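; BP_ShapeParent is a shape actor that builds a figure of clickable points joined by lines from its spline.
; On BeginPlay it spawns a BP_ClickableLocation at each spline point, then BP_StretchLines actors between paired points.
; Each Pairings string encodes neighbours as single-digit, 1-based point numbers.
; CreateNewEndPoint adds another point at the first spline position when the game mode's BackToStart is set; construction-script spline-mesh code is disconnected.
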(event `CreateNewEndPoint`
  (if (`/Game/TopDown/Blueprints/BP_TopDownGameMode.BackToStart` (`self.GamemodeRef`))
    (bind _returnvalue (`|SpawnActorFromClass` "/Game/Blueprints/BP_ClickableLocation.BP_ClickableLocation_C" (`KismetMathLibrary.MakeTransform` (`SplineComponent.GetLocationAtSplinePoint` (`self.Spline`) 0 "Local")) "Undefined" "MultiplyWithRoot" null self "" 0 null))
    (`KismetArrayLibrary.Array_Add` (`self.ClickablePoints`) _returnvalue)
    (`/Engine/EditorBlueprintResources/StandardMacros.IncrementInt` (`self.TotalPoints`))))

(event `self.ReceiveBeginPlay`
  (bind _asbp_top_down_game_mode (cast `/Game/TopDown/Blueprints/BP_TopDownGameMode` (`GameplayStatics.GetGameMode`)))
  (set `self.GamemodeRef` _asbp_top_down_game_mode)
  (`self.PopulateSpline`)
  (`KismetSystemLibrary.Delay` 1.0))

(event `PopulateSpline`
  (bind _spline (`self.Spline`))
  (for _index (range (`SplineComponent.GetNumberOfSplinePoints` _spline))
    (bind _returnvalue (`|SpawnActorFromClass` "/Game/Blueprints/BP_ClickableLocation.BP_ClickableLocation_C" (`KismetMathLibrary.MakeTransform` (`.Position` (break `SplinePoint` (`SplineComponent.GetSplinePointAt` _spline _index "World")))) "Undefined" "MultiplyWithRoot" null self (`|GetArrayItem` (`self.Pairings`) _index) (+ _index 1) null))
    (`KismetArrayLibrary.Array_Add` (`self.ClickablePoints`) _returnvalue)
    (`/Engine/EditorBlueprintResources/StandardMacros.DoOnce` false))
  (set `self.TotalPoints` (`KismetArrayLibrary.Array_Length` (`self.ClickablePoints`)))
  (`self.CreateLines`))

(event `CreateLines`
  (for _array_element (`self.ClickablePoints`)
    (bind _pairedwith (`/Game/Blueprints/BP_ClickableLocation.PairedWith` _array_element))
    (bind _returnvalue (`KismetStringLibrary.Len` _pairedwith))
    (`KismetSystemLibrary.PrintString` (`KismetStringLibrary.Conv_IntToString` _returnvalue))
    (for _index (range _returnvalue)
      (bind _returnvalue_2 (`SceneComponent.K2_GetComponentLocation` (`/Game/Blueprints/BP_ClickableLocation.Cube` _array_element)))
      (`KismetSystemLibrary.PrintString` (`KismetStringLibrary.Conv_VectorToString` _returnvalue_2))
      (bind _returnvalue_3 (`SceneComponent.K2_GetComponentLocation` (`Actor.RootComponent` (`|GetArrayItem` (`self.ClickablePoints`) (- (`KismetStringLibrary.Conv_StringToInt` (`KismetStringLibrary.GetSubstring` _pairedwith _index)) 1)))))
      (`KismetSystemLibrary.PrintString` (`KismetStringLibrary.Conv_VectorToString` _returnvalue_3))
      (`|SpawnActorFromClass` "/Game/Blueprints/BP_StretchLines.BP_StretchLines_C" (`KismetMathLibrary.MakeTransform` (0.0 0.0 0.0)) "Undefined" "MultiplyWithRoot" null _returnvalue_2 _returnvalue_3 null))))

(fn `UserConstructionScript`)