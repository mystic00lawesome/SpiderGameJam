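; BP_ShapeSpawner is a placeable actor that spawns the current round's shape at its own location.
; On BeginPlay it casts the game mode to BP_TopDownGameMode and binds to its round start and cleanup dispatchers.
; Round start spawns the game mode's ShapeToSpawn class and stores the instance, which cleanup then destroys.
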(event `self.ReceiveBeginPlay`
  (bind _gamemoderef (`self.GameModeRef`))
  (bind _asbp_top_down_game_mode (cast `/Game/TopDown/Blueprints/BP_TopDownGameMode` (`GameplayStatics.GetGameMode`)))
  (set `self.GameModeRef` _asbp_top_down_game_mode)
  (add `/Game/TopDown/Blueprints/BP_TopDownGameMode.StartRoundLol` _gamemoderef (delegate `SpawnShape`))
  (add `/Game/TopDown/Blueprints/BP_TopDownGameMode.CleanupRoundLol` _gamemoderef (delegate `CleanupRound`)))

(event `SpawnShape`
  (bind _returnvalue (`|SpawnActorFromClass` (`/Game/TopDown/Blueprints/BP_TopDownGameMode.ShapeToSpawn` (`self.GameModeRef`)) (`KismetMathLibrary.MakeTransform` (`SceneComponent.K2_GetComponentLocation` (`self.DefaultSceneRoot`))) "Undefined" "MultiplyWithRoot" null null))
  (set `self.Shape` _returnvalue))

(event `CleanupRound`
  (`self.K2_DestroyActor` (`self.Shape`)))

(fn `UserConstructionScript`)