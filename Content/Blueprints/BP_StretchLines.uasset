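; BP_StretchLines is an actor that draws a stretched line, using a web projection material, between SplineStart and SplineEnd.
; On BeginPlay it builds a world-space spline from those points, then adds a spline mesh component per segment, matched to the spline's locations and tangents.
; It also binds to BP_TopDownGameMode's round cleanup event and destroys itself when that fires.
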(event `self.ReceiveBeginPlay`
  (bind _locationarray (`self.LocationArray`))
  (bind _spline (`self.Spline`))
  (bind _asbp_top_down_game_mode (cast `/Game/TopDown/Blueprints/BP_TopDownGameMode` (`GameplayStatics.GetGameMode`)))
  (set `self.As BP Top Down Game Mode` _asbp_top_down_game_mode)
  (`KismetArrayLibrary.Array_Add` _locationarray (`self.SplineStart`))
  (`KismetArrayLibrary.Array_Add` _locationarray (`self.SplineEnd`))
  (`SplineComponent.SetSplinePoints` (`self.Spline`) (`self.LocationArray`) "World" true)
  (for _index (range (+ (- (`SplineComponent.GetNumberOfSplinePoints` (`self.Spline`)) 2) 1))
    (bind _returnvalue (`AddComponent|NODE_AddSplineMeshComponent-1`))
    (`SplineMeshComponent.SetForwardAxis` _returnvalue "X" true)
    (`PrimitiveComponent.SetMaterial` _returnvalue 0 "/Game/Materials/M_WebProjection.M_WebProjection")
    (bind (_location _tangent) (`SplineComponent.GetLocationAndTangentAtSplinePoint` _spline _index "Local"))
    (bind (_location_2 _tangent_2) (`SplineComponent.GetLocationAndTangentAtSplinePoint` _spline (+ _index 1) "Local"))
    (`SplineMeshComponent.SetStartAndEnd` _returnvalue _location _tangent _location_2 _tangent_2 true)
    (`SceneComponent.K2_AttachToComponent` _returnvalue (`self.DefaultSceneRoot`) "None" "KeepWorld" "KeepWorld" "KeepWorld" true))
  (add `/Game/TopDown/Blueprints/BP_TopDownGameMode.CleanupRoundLol` (`self.As BP Top Down Game Mode`) (delegate `asfvadfbaebt`)))

(event `asfvadfbaebt`
  (`self.K2_DestroyActor`))

(fn `UserConstructionScript`)