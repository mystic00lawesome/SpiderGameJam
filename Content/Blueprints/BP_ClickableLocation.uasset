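; BP_ClickableLocation is a point in a parent shape's pairing puzzle that the top-down character moves onto.
; On BeginPlay it splits its PairedWith string into single-digit integers stored in PairedWithArray.
; When the character overlaps its cube, it re-enables movement and scans the parent's ClickablePoints for any non-empty pair arrays.
; If none remain, it sets the round as won through the parent's game mode reference.
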(event `self.ReceiveBeginPlay`
  (for _index (range (`KismetStringLibrary.Len` (`self.PairedWith`)))
    (`KismetArrayLibrary.Array_Add` (`self.PairedWithArray`) (`KismetStringLibrary.Conv_StringToInt` (`KismetStringLibrary.GetSubstring` (`self.PairedWith`) _index)))))

(event `self.Cube.OnComponentBeginOverlap`
  (params (OverlappedComponent :type "PrimitiveComponent Object Reference") (OtherActor :type "Actor Object Reference") (OtherComp :type "PrimitiveComponent Object Reference") (OtherBodyIndex :type Integer) (bFromSweep :type Boolean) (SweepResult :type "HitResult Structure (by ref)"))
  (bind _parentshape (`self.ParentShape`))
  (bind _parentshape_2 (`self.ParentShape`))
  (bind _asbp_top_down_character (cast `/Game/TopDown/Blueprints/BP_TopDownCharacter` OtherActor))
  (set `/Game/TopDown/Blueprints/BP_TopDownCharacter.CanMove` true _asbp_top_down_character)
  (set `/Game/Blueprints/BP_ShapeParent.StillPairsToComplete` false _parentshape)
  (for _array_element (`/Game/Blueprints/BP_ShapeParent.ClickablePoints` _parentshape)
    (if (> (`KismetArrayLibrary.Array_Length` (`/Game/Blueprints/BP_ClickableLocation.PairedWithArray` _array_element)) 0)
      (set `/Game/Blueprints/BP_ShapeParent.StillPairsToComplete` true (`self.ParentShape`))
      (`KismetSystemLibrary.PrintString` "still pairs")))
  (if (not (`/Game/Blueprints/BP_ShapeParent.StillPairsToComplete` _parentshape_2))
    (`/Game/TopDown/Blueprints/BP_TopDownGameMode.SetRoundWon` (`/Game/Blueprints/BP_ShapeParent.GamemodeRef` _parentshape_2) true)))

(fn `UserConstructionScript`)