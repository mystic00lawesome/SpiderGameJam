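; BP_SmallSpiders is a small spider actor that supports the game's arachnophobia mode by changing its appearance.
; On BeginPlay it binds SwitchToPhobia to the arachnophobia mode event.
; That handler reads the mode from BP_TopDownGameMode and sets the Spider mesh and scale, showing a spider in Standard Mode and a mustard mesh in Phobia Mode.
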(event `self.ReceiveBeginPlay`
  (add `self.ArachnophobiaMode` (delegate `SwitchToPhobia`)))

(event `SwitchToPhobia`
  (bind _asbp_top_down_game_mode (cast `/Game/TopDown/Blueprints/BP_TopDownGameMode` (`GameplayStatics.GetGameMode`)))
  (switch `/Game/E_ArachnophobiaMode` (`/Game/TopDown/Blueprints/BP_TopDownGameMode.E_GameMode` _asbp_top_down_game_mode)
    (:`NewEnumerator0`
      (`StaticMeshComponent.SetStaticMesh` (`self.Spider`) "/Game/Enviro/SM_Small_Spider.SM_Small_Spider")
      (`SceneComponent.SetWorldScale3D` (`self.Spider`) (4.8 4.8 4.8)))
    (:`NewEnumerator1`
      (`StaticMeshComponent.SetStaticMesh` (`self.Spider`) "/Game/Enviro/SM_Mustard.SM_Mustard")
      (`SceneComponent.SetWorldScale3D` (`self.Spider`) (0.5 0.5 0.5)))))

(fn `UserConstructionScript`)